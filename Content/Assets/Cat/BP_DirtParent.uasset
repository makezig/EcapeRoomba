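; BP_DirtParent is a dirt actor, apparently a base class, that the player cleans by touching it.
; On actor overlap it prints a debug message, and if the other actor is the player character it sets IsTouched and destroys itself.
; CleanCounter runs after the destroy call, incrementing and printing Cleaned, a variable on the dirt actor itself rather than a shared tally.
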(event OnComponentBeginOverlap(Box)
  (params (OverlappedComponent :type Primitive%20Component%20Object%20Reference) (OtherActor :type Actor%20Object%20Reference) (OtherComp :type Primitive%20Component%20Object%20Reference) (OtherBodyIndex :type Integer) (bFromSweep :type Boolean) (SweepResult :type Hit%20Result%20Structure%20%28by%20ref%29)))

(event EventBeginPlay)

(event Collision|EventActorBeginOverlap
  (params (OtherActor :type Actor%20Object%20Reference))
  (Development|PrintString "Triggered")
  (if (== OtherActor (Game|GetPlayerCharacter 0))
    (Variables|Default|SetIsTouched true)
    (Actor|DestroyActor)
    (CallFunction|CleanCounter)))

(event EventTick
  (params (DeltaSeconds :type Float%20%28single-precision%29)))

(fn ConstructionScript)

(fn CleanCounter
  (bind _result (Math|Integer|IncrementInt (Variables|Default|GetCleaned))
    (:%20%20
      (bind _output_get (Variables|Default|SetCleaned _result))
      (Development|PrintString (Utilities|String|ToString(Integer) _output_get)))))