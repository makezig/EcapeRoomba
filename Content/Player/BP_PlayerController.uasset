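; Player controller Blueprint that switches possession between the Character actors in the level.
; On BeginPlay it builds a roster with GetAllActorsOfClass and records the player's starting character as the current one.
; The In_ToggleVacuum input action calls NextCharacter, which possesses the next roster entry and wraps to the first at the end.
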(event Input|EnhancedActionEvents|EnhancedInputActionIn_ToggleVacuum
  (params (ActionValue :type Boolean) (ElapsedSeconds :type Float%20%28double-precision%29) (TriggeredSeconds :type Float%20%28double-precision%29) (InputAction :type Input%20Action%20Object%20Reference :default "/Game/Input/In_ToggleVacuum.In_ToggleVacuum"))
  (:Started
    (CallFunction|NextCharacter)))

(event EventBeginPlay
  (bind _outactors (Actor|GetAllActorsOfClass "/Script/Engine.Character"))
  (Variables|Default|SetCharacterRoster _outactors)
  (bind _ascharacter (Utilities|Casting|CastToCharacter (Game|GetPlayerCharacter 0)))
  (Variables|Default|SetcurrentCharacter _ascharacter))

(fn ConstructionScript)

(fn NextCharacter
  (LocalVariables|SetLocal_Index (Utilities|Array|FindItem (Variables|Default|GetCharacterRoster) (Variables|Default|GetcurrentCharacter)))
  (bind _output_get (LocalVariables|SetLocal_Index (Math|Integer|SelectInt (+ (Utilities|Array|FindItem (Variables|Default|GetCharacterRoster) (Variables|Default|GetcurrentCharacter)) 1) 0 (Utilities|Array|IsValidIndex (Variables|Default|GetCharacterRoster) (+ (Utilities|Array|FindItem (Variables|Default|GetCharacterRoster) (Variables|Default|GetcurrentCharacter)) 1)))))
  (bind _output_get_2 (Variables|Default|SetcurrentCharacter (Utilities|Array|Get(acopy) (Variables|Default|GetCharacterRoster) _output_get)))
  (Pawn|Possess _output_get_2))